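; Drivable bulldozer pawn that the player can enter, drive, operate and leave via a timed hold with camera fade.
; Axis input feeds Chaos-style movement and the AnimBP's arm and loader angles, which rotate collision components.
; Landscape overlap blocks negative arm and loader input and, with forward motion, fills a rubble material parameter; tilting the loader empties it with Niagara particles.
; Tick also updates exhaust, engine audio, brake and reverse lights.
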(event `self.ReceiveBeginPlay`
  (`|ExecutionSequence`
    (:`then_0`
      ;[1 1 1] Initialization
      (bind _asab_bulldozer_01_01 (cast `/Game/ConstructionSite/Vehicle/Bulldozer_01/Blueprints/AB_Bulldozer_01_01` (`SkeletalMeshComponent.GetAnimInstance` (`self.Mesh`))))
      (set `self.VehicleAnimBP` _asab_bulldozer_01_01))
    (:`then_1`
      (`/Game/ConstructionSite/Vehicle/Bulldozer_01/Blueprints/BP_CameraSwitcher_01_01.SetCameras` (`self.CameraSwitcher`) (`|MakeArray` (`self.OutsideCam`) (`self.InsideCam`) (`self.WheelCam`))))
    (:`then_2`
      (`self.SetupDynamicMaterials`)
      (`self.SetEmissiveOnMaterial` (`self.StopLights`))
      (`self.SetEmissiveOnMaterial` (`self.HeadLights`))
      (`self.SetEmissiveOnMaterial` (`self.ReverseLights`)))
    (:`then_3`
      (`ActorComponent.SetActive` (`self.EngineSound`) false true))))

(event `InputAxis|ArmSteering`
  (params (AxisValue :type "Float (single-precision)"))
  (bind _vehicleanimbp (`self.VehicleAnimBP`))
  ;[1 1 1] Arm animations
  (if (> AxisValue 0.0)
    (`/Game/ConstructionSite/Vehicle/Bulldozer_01/Blueprints/AB_Bulldozer_01_01.AddArmInput` _vehicleanimbp (* AxisValue (`self.ArmSpeedScale`)) 0.0 50.0 :!label _label)
    (`SceneComponent.K2_SetRelativeRotation` (`self.CollisionArm`) (`KismetMathLibrary.MakeRotator` 0.0 (`/Game/ConstructionSite/Vehicle/Bulldozer_01/Blueprints/AB_Bulldozer_01_01.ArmAngle` _vehicleanimbp)) false false)
    (elif (not (`self.isGroundBlocked`))
      (`/Engine/EditorBlueprintResources/StandardMacros.IsValid` _vehicleanimbp
        (:`Is Valid`
          (goto _label))))))

(event `InputAxis|Turn`
  (params (AxisValue :type "Float (single-precision)"))
  ;[1 1 1] Camera rotation
  (`SceneComponent.K2_AddRelativeRotation` (`self.OutsideCamera`) (`KismetMathLibrary.MakeRotator` 0.0 0.0 AxisValue) false false)
  (`SceneComponent.K2_AddRelativeRotation` (`self.InsideCamera`) (`KismetMathLibrary.MakeRotator` 0.0 0.0 AxisValue) false false))

(event `InputAction|ToggleCamera`
  (params (Key :type "Key Structure"))
  ;[1 1 1] Camera toggle
  (:`Pressed`
    (`/Game/ConstructionSite/Vehicle/Bulldozer_01/Blueprints/BP_CameraSwitcher_01_01.ActivateNext` (`self.CameraSwitcher`))))

(event `InputAxis|LoaderSteering`
  (params (AxisValue :type "Float (single-precision)"))
  (bind _vehicleanimbp (`self.VehicleAnimBP`))
  ;[1 1 1] Arm animations
  (if (> AxisValue 0.0)
    (`/Game/ConstructionSite/Vehicle/Bulldozer_01/Blueprints/AB_Bulldozer_01_01.AddLoaderInput` _vehicleanimbp (* AxisValue (`self.LoaderSpeedScale`)) -120.0 20.0 :!label _label_2)
    (`SceneComponent.K2_SetRelativeRotation` (`self.CollisionLoader`) (`KismetMathLibrary.MakeRotator` 0.0 (`/Game/ConstructionSite/Vehicle/Bulldozer_01/Blueprints/AB_Bulldozer_01_01.LoaderAngle` _vehicleanimbp)) false false)
    (elif (not (`self.isGroundBlocked`))
      (`/Engine/EditorBlueprintResources/StandardMacros.IsValid` _vehicleanimbp
        (:`Is Valid`
          (goto _label_2))))))

(event `InputAxis|MoveForward`
  (params (AxisValue :type "Float (single-precision)"))
  (bind _vehiclemovementcomponent (`self.VehicleMovementComponent`))
  ;[1 1 1] Driving
  (if (> AxisValue 0.0)
    (`ChaosVehicleMovementComponent.SetThrottleInput` _vehiclemovementcomponent AxisValue)
    (`ChaosVehicleMovementComponent.SetBrakeInput` _vehiclemovementcomponent 0.0)
    (`self.CalculateBreakingInput`)
    (else
      (`ChaosVehicleMovementComponent.SetThrottleInput` _vehiclemovementcomponent 0.0)
      (`ChaosVehicleMovementComponent.SetBrakeInput` _vehiclemovementcomponent (`KismetMathLibrary.Abs` AxisValue)))))

(event `InputAxis|LookUp`
  (params (AxisValue :type "Float (single-precision)"))
  (bind _returnvalue (* AxisValue -1.0))
  ;[1 1 1] Camera rotation
  (`self.AddCameraPitchClamped` (`self.OutsideCamera`) _returnvalue -70.0)
  (`self.AddCameraPitchClamped` (`self.InsideCamera`) _returnvalue -70.0 40.0))

(event `InputAction|ToggleLight`
  (params (Key :type "Key Structure"))
  (bind _topright (`self.TopRight`))
  (bind _returnvalue (`SceneComponent.IsVisible` _topright))
  ;[1 1 1] Light toggle
  (:`Released`
    (`SceneComponent.ToggleVisibility` _topright false)
    (`SceneComponent.ToggleVisibility` (`self.DownRight`) false)
    (`SceneComponent.ToggleVisibility` (`self.TopLeft2`) false)
    (`SceneComponent.ToggleVisibility` (`self.DownLeft`) false)
    (`SceneComponent.ToggleVisibility` (`self.RearLeft`) false)
    (`SceneComponent.ToggleVisibility` (`self.RearRight`) false)
    (`SceneComponent.ToggleVisibility` (`self.Cabine`) false)
    (`self.SetEmissiveOnMaterial` (`self.HeadLights`) _returnvalue)
    (`self.SetEmissiveOnMaterial` (`self.ReverseLights`) _returnvalue)))

(event `InputAxis|MoveRight`
  (params (AxisValue :type "Float (single-precision)"))
  ;[1 1 1] Driving
  (`ChaosVehicleMovementComponent.SetSteeringInput` (`self.VehicleMovementComponent`) AxisValue)
  (`/Game/ConstructionSite/Vehicle/Bulldozer_01/Blueprints/AB_Bulldozer_01_01.SetSteeringWheelInput` (`self.VehicleAnimBP`) AxisValue -130.0 130.0))

(event `self.ReceiveTick`
  (params (DeltaSeconds :type "Float (single-precision)"))
  (bind _niagararubbleparticle (`self.NiagaraRubbleParticle`))
  (bind _returnvalue (`ChaosVehicleMovementComponent.GetForwardSpeed` (`self.VehicleMovementComponent`)))
  (bind _loaderangle (`/Game/ConstructionSite/Vehicle/Bulldozer_01/Blueprints/AB_Bulldozer_01_01.LoaderAngle` (`self.VehicleAnimBP`)))
  ;[1 1 1] Update effects
  (`|ExecutionSequence`
    (:`then_0`
      (`self.UpdateExhaustIntensity`))
    (:`then_1`
      (`self.UpdateReverseGearEffects`))
    (:`then_2`
      (`self.UpdateBrakeLights`))
    (:`then_3`
      (`self.UpdateEngineSound`))
    (:`then_4`
      ;[1 1 1] Loader rubble In
      (if (> _returnvalue 0.0)
        (if (`self.isGroundBlocked`)
          (if (not (`self.isRubbleFalling`))
            (set `self.RubbleValue` (`KismetMathLibrary.FClamp` (+ (`self.RubbleValue`) (* (* DeltaSeconds 0.1) (`KismetMathLibrary.FClamp` (/ _returnvalue 300.0) 0.0 2.0)))))
            (`MaterialInstanceDynamic.SetScalarParameterValue` (`self.RubbleMID`) "Rubble" (`KismetMathLibrary.MultiplyMultiply_FloatFloat` (`self.RubbleValue`) 0.7))))))
    (:`then_5`
      ;[1 1 1] Loader rubble Out
      (if (> (`self.RubbleValue`) 0.0)
        (if (< _loaderangle -50.0)
          (`ActorComponent.Activate` _niagararubbleparticle false)
          (set `self.isRubbleFalling` true)
          (set `self.RubbleValue` (`KismetMathLibrary.FClamp` (- (`self.RubbleValue`) (* (* DeltaSeconds 0.5) (- 1.0 (`KismetMathLibrary.FClamp` (/ (- 120.0 (`KismetMathLibrary.Abs` _loaderangle)) 70.0)))))))
          (`MaterialInstanceDynamic.SetScalarParameterValue` (`self.RubbleMID`) "Rubble" (`self.RubbleValue`))
          (else
            (`ActorComponent.Deactivate` _niagararubbleparticle :!label _label_3)
            (set `self.isRubbleFalling` false)))
        (else
          (goto _label_3))))))

(event `InputAction|CameraZoomIn`
  (params (Key :type "Key Structure"))
  ;[1 1 1] Camera zoom in/out
  (:`Pressed`
    (`self.CameraZoom` -100.0 700.0 1400.0)))

(event `InputAction|Jump`
  (params (Key :type "Key Structure"))
  (bind _vehiclemovementcomponent (`self.VehicleMovementComponent`))
  ;[1 1 1] Driving
  (:`Pressed`
    (`ChaosVehicleMovementComponent.SetHandbrakeInput` _vehiclemovementcomponent true)
    (set `self.HandBrake` true))
  (:`Released`
    (`ChaosVehicleMovementComponent.SetHandbrakeInput` _vehiclemovementcomponent false)
    (set `self.HandBrake` false)))

(event `InputAction|CameraZoomOut`
  (params (Key :type "Key Structure"))
  ;[1 1 1] Camera zoom in/out
  (:`Pressed`
    (`self.CameraZoom` 100.0 700.0 1400.0)))

(event `InputAction|ToggleControls`
  (params (Key :type "Key Structure"))
  ;[1 1 1] Controls - UI toggle
  (:`Pressed`
    (`/Game/ConstructionSite/Vehicle/Bulldozer_01/UI/B_HUDVehicle_01_01.ToggleControls` (`self.VehicleUI`))))

(event `InputAction|Interact`
  (params (Key :type "Key Structure"))
  (bind _vehicleui (`self.VehicleUI`))
  (bind _playercameramanager (`PlayerController.PlayerCameraManager` (cast `PlayerController` (`self.GetController`) :!pure true)))
  ;[1 1 1] Handle player exit
  (:`Pressed`
    (bind _returnvalue (`KismetSystemLibrary.K2_SetTimerDelegate` (delegate `ExitVehicle`) (`self.ExitDelay`)))
    (set `self.ExitTimer` _returnvalue)
    ;[1 1 1] Fade out during exiting
    (`PlayerCameraManager.StartCameraFade` :`self` _playercameramanager :`ToAlpha` 1.0 :`Duration` (`self.ExitDelay`) :`bHoldWhenFinished` true)
    (`/Engine/EditorBlueprintResources/StandardMacros.IsValid` _vehicleui
      (:`Is Valid`
        (`/Game/ConstructionSite/Vehicle/Bulldozer_01/UI/B_HUDVehicle_01_01.StartProgress` _vehicleui (`self.ExitDelay`)))))
  (:`Released`
    (`KismetSystemLibrary.K2_ClearAndInvalidateTimerHandle` (`self.ExitTimer`))
    (if (not (`self.IsExitCompleted`))
      (`PlayerCameraManager.StopCameraFade` _playercameramanager)
      (`/Engine/EditorBlueprintResources/StandardMacros.IsValid` _vehicleui
        (:`Is Valid`
          (`/Game/ConstructionSite/Vehicle/Bulldozer_01/UI/B_HUDVehicle_01_01.StopProgress` _vehicleui))))))

(event `ExitVehicle`
  (bind _vehicleui (`self.VehicleUI`))
  ;[1 1 1] Player spawning on exit
  (`|ExecutionSequence`
    (:`then_0`
      (set `self.IsExitCompleted` true)
      (`/Engine/EditorBlueprintResources/StandardMacros.IsValid` (`self.Player`)
        (:`Is Valid`
          (`self.K2_SetActorLocation` (`self.Player`) (`KismetMathLibrary.TransformLocation` (`self.GetTransform`) (`self.PlayerExitLocation`)) false true)
          (`KismetSystemLibrary.Delay` (`self.FadeDelay`))
          (`Controller.Possess` (`self.GetController`) (`self.Player`))
          (set `self.Player` null))))
    (:`then_1`
      (`/Engine/EditorBlueprintResources/StandardMacros.IsValid` _vehicleui
        (:`Is Valid`
          (`/Game/ConstructionSite/Vehicle/Bulldozer_01/UI/B_HUDVehicle_01_01.StopProgress` _vehicleui))))
    (:`then_2`
      (`GameplayStatics.PlaySoundAtLocation` "/Game/ConstructionSite/Effects/Sounds_01/S_EngineOff_01_01.S_EngineOff_01_01" (`SceneComponent.K2_GetComponentLocation` (`self.EngineSound`)) (struct) 1.0 1.0 0.0 null null null null))
    (:`then_3`
      (`ChaosVehicleMovementComponent.SetParked` (`self.VehicleMovementComponent`) true))))

(event `self.ReceivePossessed`
  (params (NewController :type "Controller Object Reference"))
  ;[1 1 1] On enter vehicle
  (`|ExecutionSequence`
    (:`then_0`
      (bind _asplayer_controller (cast `PlayerController` NewController))
      (`PlayerCameraManager.StartCameraFade` :`self` (`PlayerController.PlayerCameraManager` _asplayer_controller) :`FromAlpha` 1.0 :`Duration` (`self.FadeDelay`) :`bHoldWhenFinished` true)
      (`self.CreateVehicleUI`)
      ;[1 1 1] Show Controls UI when entered vehicle - only once
      ; By default, UI should be hidden
      (`/Game/ConstructionSite/Vehicle/Bulldozer_01/UI/B_HUDVehicle_01_01.SetControlsVisibility` (`self.VehicleUI`) (`self.IsFirstEntry`))
      (set `self.IsFirstEntry` false))
    (:`then_1`
      (`SceneComponent.K2_SetRelativeRotation` (`self.OutsideCamera`) (`self.InitialCameraRotation`) false false)
      (`SceneComponent.K2_SetRelativeRotation` :`self` (`self.InsideCamera`)))
    (:`then_2`
      (`/Game/ConstructionSite/Vehicle/Bulldozer_01/Blueprints/BP_CameraSwitcher_01_01.ActivateFirst` (`self.CameraSwitcher`)))
    (:`then_3`
      (set `self.IsExitCompleted` false))
    (:`then_4`
      (`ActorComponent.SetActive` (`self.EngineSound`) true false))
    (:`then_5`
      (`ChaosVehicleMovementComponent.SetParked` (`self.VehicleMovementComponent`) false))))

(event `self.ReceiveUnpossessed`
  (params (OldController :type "Controller Object Reference"))
  ;[1 1 1] On exit vehicle
  (`self.RemoveVehicleUI`)
  (`ChaosVehicleMovementComponent.SetHandbrakeInput` (`self.VehicleMovementComponent`) true)
  (`ActorComponent.SetActive` (`self.EngineSound`) false true))

(event `self.GroundBlocker.OnComponentBeginOverlap`
  (params (OverlappedComponent :type "PrimitiveComponent Object Reference") (OtherActor :type "Actor Object Reference") (OtherComp :type "PrimitiveComponent Object Reference") (OtherBodyIndex :type Integer) (bFromSweep :type Boolean) (SweepResult :type "HitResult Structure (by ref)"))
  ;[1 1 1] Handle ground collision
  (cast `Landscape` OtherActor)
  (set `self.isGroundBlocked` true))

(event `self.GroundBlocker.OnComponentEndOverlap`
  (params (OverlappedComponent :type "PrimitiveComponent Object Reference") (OtherActor :type "Actor Object Reference") (OtherComp :type "PrimitiveComponent Object Reference") (OtherBodyIndex :type Integer))
  ;[1 1 1] Handle ground collision
  (cast `Landscape` OtherActor)
  (set `self.isGroundBlocked` false))

(fn `AddArmInput`)

(fn `AddCameraPitchClamped`
  (params (SpringArm :type "SpringArmComponent Object Reference (by ref)") (Value :type "Float (double-precision) (by ref)") (Min :type "Float (double-precision)") (Max :type "Float (double-precision)"))
  (locals (inputRotation :type "Float (double-precision)"))
  (bind (_returnvalue_roll _returnvalue_pitch) (`KismetMathLibrary.BreakRotator` (`SceneComponent.K2_GetComponentRotation` SpringArm)))
  (set `local.inputRotation` _returnvalue_pitch)
  (`SceneComponent.K2_AddRelativeRotation` SpringArm (`KismetMathLibrary.MakeRotator` 0.0 (`KismetMathLibrary.SelectFloat` Value 0.0 (`KismetMathLibrary.InRange_FloatFloat` (+ Value _returnvalue_pitch) Min Max))) false false))

(fn `AddLoaderInput`)

(fn `CalculateBreakingInput`
  (bind _returnvalue (`self.GetInputAxisValue`))
  (bind _returnvalue_2 (`ChaosVehicleMovementComponent.GetCurrentGear` (`self.VehicleMovementComponent`)))
  (set `self.Brakeing` (or (and (< _returnvalue 0.0) (>= _returnvalue_2 0)) (and (> _returnvalue 0.0) (< _returnvalue_2 0)))))

(fn `CameraZoom`
  (params (amount :type "Float (double-precision)") (min :type "Float (double-precision)") (max :type "Float (double-precision)"))
  (bind _outsidecamera (`self.OutsideCamera`))
  (set `SpringArmComponent.TargetArmLength` (`KismetMathLibrary.FClamp` (+ amount (`SpringArmComponent.TargetArmLength` _outsidecamera)) min max) _outsidecamera))

(fn `CreateVehicleUI`
  (`/Engine/EditorBlueprintResources/StandardMacros.IsValid` (`self.VehicleUI`)
    (:`Is Valid`
      _)
    (:`Is Not Valid`
      (bind _returnvalue (`|CreateWidget` "/Game/ConstructionSite/Vehicle/Bulldozer_01/UI/B_HUDVehicle_01_01.B_HUDVehicle_01_01_C"))
      (bind _output_get (set `self.VehicleUI` _returnvalue))))
  (`UserWidget.AddToViewport` _output_get 0))

(fn `Get RPMNormalized`
  (params (MovementComponent :type "ChaosVehicleMovementComponent Object Reference"))
  (returns (NormalizedRPM :type "Float (double-precision)"))
  (bind _aschaos_wheeled_vehicle_movement_component (cast `ChaosWheeledVehicleMovementComponent` MovementComponent)
    (:`then`
      (return (`KismetMathLibrary.FClamp` (/ (`self.GetEngineRotationSpeed` _aschaos_wheeled_vehicle_movement_component) (`ChaosWheeledVehicleMovementComponent.GetEngineMaxRotationSpeed` _aschaos_wheeled_vehicle_movement_component)))))
    (:`CastFailed`
      (return 0.0))))

(fn `RemoveVehicleUI`
  (bind _vehicleui (`self.VehicleUI`))
  (`/Engine/EditorBlueprintResources/StandardMacros.IsValid` _vehicleui
    (:`Is Valid`
      (`Widget.RemoveFromParent` _vehicleui))))

(fn `SetEmissiveOnMaterial`
  (params (Material :type "MaterialInstanceDynamic Object Reference") (IsOn :type Boolean))
  (bind _returnvalue (`MaterialInstanceDynamic.K2_GetVectorParameterValue` Material (`self.EmissiveParameterName`)))
  (`MaterialInstanceDynamic.SetVectorParameterValue` Material (`self.EmissiveParameterName`) (make `LinearColor` (break `LinearColor` _returnvalue) (`.G` (break `LinearColor` _returnvalue)) (`.B` (break `LinearColor` _returnvalue)) (select `bool` IsOn :`true` 1.0))))

(fn `SetEmmisiveIntensityOnMaterial`
  (params (Material :type "MaterialInstanceDynamic Object Reference") (Intensity :type "Float (double-precision)"))
  (bind _returnvalue (`MaterialInstanceDynamic.K2_GetVectorParameterValue` Material (`self.EmissiveParameterName`)))
  (`MaterialInstanceDynamic.SetVectorParameterValue` Material (`self.EmissiveParameterName`) (make `LinearColor` (break `LinearColor` _returnvalue) (`.G` (break `LinearColor` _returnvalue)) (`.B` (break `LinearColor` _returnvalue)) Intensity)))

(fn `SetReverseLight`
  (params (IsVisible :type Boolean))
  (bind _reverselight (`self.ReverseLight`))
  (if (!= IsVisible (`SceneComponent.bVisible` _reverselight))
    (`SceneComponent.SetVisibility` _reverselight IsVisible false)))

(fn `SetReverseSound`
  (params (IsPalying :type Boolean))
  (`AudioComponent.SetBoolParameter` (`self.EngineSound`) "IsReversing" IsPalying))

(fn `SetupDynamicMaterials`
  (bind _mesh (`self.Mesh`))
  (`|ExecutionSequence`
    (:`then_0`
      (bind _returnvalue (`PrimitiveComponent.CreateDynamicMaterialInstance` _mesh 3 "/Game/ConstructionSite/Environment/Bulldozer_01/mi_BulldozerLights_01_01_ON.mi_BulldozerLights_01_01_ON" "None"))
      (set `self.HeadLights` _returnvalue))
    (:`then_1`
      (bind _returnvalue_2 (`PrimitiveComponent.CreateDynamicMaterialInstance` _mesh 8 "/Game/ConstructionSite/Environment/Bulldozer_01/mi_BulldozerLights_01_02_ON.mi_BulldozerLights_01_02_ON" "None"))
      (set `self.StopLights` _returnvalue_2))
    (:`then_2`
      (bind _returnvalue_3 (`PrimitiveComponent.CreateDynamicMaterialInstance` _mesh 7 "/Game/ConstructionSite/Environment/Bulldozer_01/mi_BulldozerLights_02_01_ON.mi_BulldozerLights_02_01_ON" "None"))
      (set `self.ReverseLights` _returnvalue_3))))

(fn `UpdateBrakeLights`
  (`self.SetEmmisiveIntensityOnMaterial` (`self.StopLights`) (select `bool` (or (`self.Brakeing`) (`self.HandBrake`)) :`false` (select `bool` (`SceneComponent.IsVisible` (`self.RearLeft`)) :`true` (`self.ParkingLightsIntensity`)) :`true` 1.0)))

(fn `UpdateEngineSound`
  (bind _normalizedrpm (`self.Get RPMNormalized` (`self.VehicleMovementComponent`)))
  (`AudioComponent.SetFloatParameter` (`self.EngineSound`) "EnginePitch" _normalizedrpm))

(fn `UpdateExhaustIntensity`
  (bind _normalizedrpm (`self.Get RPMNormalized` (`self.VehicleMovementComponent`)))
  (`/Game/ConstructionSite/Vehicle/Bulldozer_01/Blueprints/BP_VehicleExhaust_01_01.SetIntensity` (`self.BP_VehicleExhaust`) _normalizedrpm))

(fn `UpdateReverseGearEffects`
  (bind _returnvalue (< (`ChaosVehicleMovementComponent.GetCurrentGear` (`self.VehicleMovementComponent`)) 0))
  (`self.SetReverseLight` _returnvalue)
  (`self.SetReverseSound` _returnvalue)
  (`self.SetEmissiveOnMaterial` (`self.ReverseLights`) _returnvalue))

(fn `UserConstructionScript`
  (bind _returnvalue (`PrimitiveComponent.CreateDynamicMaterialInstance` (`self.Rubble`) 0 "/Game/ConstructionSite/Effects/Vehicles_01/Materials/m_LoaderRubble_01_01.m_LoaderRubble_01_01" "None"))
  (bind _output_get (set `self.RubbleMID` _returnvalue))
  (`MaterialInstanceDynamic.SetScalarParameterValue` _output_get "Rubble" (`self.RubbleValue`)))