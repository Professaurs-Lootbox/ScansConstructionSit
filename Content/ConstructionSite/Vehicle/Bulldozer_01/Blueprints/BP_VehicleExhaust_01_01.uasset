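; Scene component that drives the Niagara exhaust effect for the construction site bulldozer.
; On BeginPlay it spawns the particle template attached to itself, keeps a reference and sets intensity to zero.
; SetIntensity maps its input through RPM-named float curves to the effect's exhaust intensity and vertical velocity parameters.
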(event `self.ReceiveBeginPlay`
  (bind _returnvalue (`NiagaraFunctionLibrary.SpawnSystemAttached` (`self.NiagaraParticleTemplate`) self "None" (0.0 0.0 0.0) (struct) "KeepRelativeOffset"))
  (set `self.NiagaraCurrentExhaust` _returnvalue)
  (`self.SetIntensity` 0.0))

(fn `SetIntensity`
  (params (Intensity :type "Float (double-precision)"))
  (`FXSystemComponent.SetFloatParameter` (`self.NiagaraCurrentExhaust`) "ExhaustIntensity" (`CurveFloat.GetFloatValue` (`self.RPM to Spawn`) Intensity))
  (`FXSystemComponent.SetVectorParameter` (`self.NiagaraCurrentExhaust`) "Velocity" (`KismetMathLibrary.MakeVector` 0.0 0.0 (`CurveFloat.GetFloatValue` (`self.RPM to Velocity`) Intensity))))