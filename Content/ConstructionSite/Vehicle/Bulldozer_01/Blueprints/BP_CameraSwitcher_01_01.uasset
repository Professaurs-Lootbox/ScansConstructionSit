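; Camera switcher Blueprint for the construction-site bulldozer that cycles through a supplied list of cameras.
; SetCameras stores the list, and ActivateCamera deactivates every entry before activating the requested one if valid.
; First, Last, Next and Previous route through ActivateByNumber, which applies modulo to the index and records the current camera.
; The modulo wraps Next past the end, but negative indices from Previous get no correction.
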(fn `ActivateByNumber`
  (params (Index :type Integer))
  (bind _cameras (`self.Cameras`))
  (bind _returnvalue (`KismetArrayLibrary.Array_Length` _cameras))
  (bind _returnvalue_2 (mod Index _returnvalue))
  (if (> _returnvalue 0)
    (bind _succeded (`self.ActivateCamera` (`|GetArrayItem` _cameras _returnvalue_2)))
    (if _succeded
      (set `self.CurrentCamera` _returnvalue_2))))

(fn `ActivateCamera`
  (params (Camera :type "CameraComponent Object Reference"))
  (returns (Succeded :type Boolean))
  (`/Engine/EditorBlueprintResources/StandardMacros.IsValid` Camera
    (:`Is Valid`
      (for _array_element (`self.Cameras`)
        (`self.SetActive` _array_element false true))
      (`self.SetActive` Camera true false)
      (return true))
    (:`Is Not Valid`
      (return false))))

(fn `ActivateFirst`
  (`self.ActivateByNumber` 0))

(fn `ActivateLast`
  (`self.ActivateByNumber` (- (`KismetArrayLibrary.Array_Length` (`self.Cameras`)) 1)))

(fn `ActivateNext`
  (`self.ActivateByNumber` (+ (`self.CurrentCamera`) 1)))

(fn `ActivatePrevious`
  (`self.ActivateByNumber` (- (`self.CurrentCamera`) 1)))

(fn `SetCameras`
  (params (Cameras :type "Array of CameraComponent Object Reference"))
  (set `self.Cameras` Cameras))