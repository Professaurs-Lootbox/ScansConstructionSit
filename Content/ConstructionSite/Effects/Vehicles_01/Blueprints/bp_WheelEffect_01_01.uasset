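; Wheel effect component for the bulldozer that drives surface particles and mud buildup on a wheel.
; BeginPlay attaches inactive Niagara systems to the vehicle mesh and puts a shared dynamic mud material on tagged meshes.
; While moving, Tick traces down for mud, water or other physical materials and activates the matching system.
; A timed mud value rises on mud, decays elsewhere, and feeds the material and a per-wheel parameter collection entry.
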(event `self.ReceiveBeginPlay`
  (bind _asbp_bulldozer_01_01 (cast `/Game/ConstructionSite/Vehicle/Bulldozer_01/bp_Bulldozer_01_01` (`self.GetOwner`)))
  (set `self.Owner` _asbp_bulldozer_01_01)
  (for _array_element (`self.NiagaraParticles`)
    (bind _returnvalue (`NiagaraFunctionLibrary.SpawnSystemAttached` _array_element (`WheeledVehiclePawn.Mesh` (`self.Owner`)) "None" (`self.RelativeLocation`) (struct) "KeepRelativeOffset" false false))
    (`KismetArrayLibrary.Array_Add` (`self.NiagaraSpawnedParticles`) _returnvalue))
  (bind _returnvalue_2 (`KismetMaterialLibrary.CreateDynamicMaterialInstance` (`self.MudMaterial`)))
  (set `self.MudMID` _returnvalue_2)
  (for _array_element_2 (`Actor.GetComponentsByTag` (`self.Owner`) "/Script/Engine.ActorComponent" (`self.MudMeshTag`))
    (bind _asstatic_mesh_component (cast `StaticMeshComponent` _array_element_2))
    (`PrimitiveComponent.SetMaterial` _asstatic_mesh_component 0 (`self.MudMID`))))

(event `self.ReceiveTick`
  (params (DeltaSeconds :type "Float (single-precision)"))
  (bind _returnvalue (`self.K2_GetComponentLocation`))
  (bind _mudvalue (`self.MudValue`))
  (bind _niagaraspawnedparticles (`self.NiagaraSpawnedParticles`))
  (bind _mudvalue_2 (`self.MudValue`))
  (bind _returnvalue_2 (/ (`self.MudValue`) 5.0))
  (bind _output (`|GetArrayItem` _niagaraspawnedparticles 1))
  (bind _output_2 (`|GetArrayItem` _niagaraspawnedparticles 2))
  (if (> (`KismetMathLibrary.Abs` (`ChaosVehicleMovementComponent.GetForwardSpeed` (`WheeledVehiclePawn.VehicleMovementComponent` (`self.Owner`)))) 50.0)
    (bind (_outhit _returnvalue_3) (`KismetSystemLibrary.LineTraceSingle` (+ _returnvalue (0.0 0.0 40.0)) (+ _returnvalue (0.0 0.0 -20.0)) "TraceTypeQuery1" true (`|MakeArray` (`self.Owner`) :!type "Actor Object Reference") "None" true (struct :`R` 1.0 :`A` 1.0) (struct :`G` 1.0 :`A` 1.0) 20.0))
    (if _returnvalue_3
      (bind (_bblockinghit _binitialoverlap _time _distance _location _impactpoint _normal _impactnormal _physmat) (`GameplayStatics.BreakHitResult` _outhit))
      (if (== _physmat "/Game/ConstructionSite/Effects/Footprints_01/PhysicalMaterials/pm_Mud_01_01.pm_Mud_01_01")
        (`self.Activate` _output false)
        (`self.Deactivate` _output_2)
        (`self.Deactivate` (`|GetArrayItem` _niagaraspawnedparticles))
        (if (< _mudvalue_2 5.0)
          (set `self.MudValue` (+ _mudvalue_2 DeltaSeconds))
          (`KismetMaterialLibrary.SetScalarParameterValue` "/Game/ConstructionSite/Effects/Vehicles_01/Materials/mpc_VehiclesParam_01_01.mpc_VehiclesParam_01_01" (`KismetStringLibrary.Conv_StringToName` (`|GetEnumeratorNameAsString` (`self.Wheel`))) _returnvalue_2 :!label _label)
          (`MaterialInstanceDynamic.SetScalarParameterValue` (`self.MudMID`) "Mud" _returnvalue_2))
        (else
          (if (== _physmat "/Game/ConstructionSite/Effects/Footprints_01/PhysicalMaterials/pm_Water_01_01.pm_Water_01_01")
            (`self.Activate` _output_2 false)
            (`self.Deactivate` _output)
            (`self.Deactivate` (`|GetArrayItem` _niagaraspawnedparticles))
            (else
              (`self.Activate` (`|GetArrayItem` _niagaraspawnedparticles) false)
              (`self.Deactivate` _output)
              (`self.Deactivate` _output_2)))
          (if (> _mudvalue 0.0)
            (set `self.MudValue` (- _mudvalue DeltaSeconds))
            (goto _label))))
      (else
        (for _array_element (`self.NiagaraSpawnedParticles`) :!label _label_2
          (`self.Deactivate` _array_element))))
    (else
      (goto _label_2))))