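; BP_DecalWater_01_01 is a water decal effect, filed with the footprint effects, that scales up from invisible when spawned.
; On BeginPlay it zeroes the decal scale, waits a configurable delay, then plays the DecalSize timeline to drive the decal's world scale.
; With UseParticle set, it first spawns a Niagara system at the decal, and the timeline only plays if that system asset is valid.
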(event `self.ReceiveBeginPlay`
  (bind _niagaraparticle (`self.NiagaraParticle`))
  (`SceneComponent.SetWorldScale3D` (`self.Decal`) (0.0 0.0 0.0))
  (`KismetSystemLibrary.Delay` (`self.Delay`))
  (if (`self.UseParticle`)
    (`/Engine/EditorBlueprintResources/StandardMacros.IsValid` _niagaraparticle
      (:`Is Valid`
        (`NiagaraFunctionLibrary.SpawnSystemAtLocation` _niagaraparticle (`SceneComponent.K2_GetComponentLocation` (`self.Decal`)))
        (bind (_direction _decalsize) (`Timeline|DecalSize` :!label _label)
          (:`Update`
            (`SceneComponent.SetWorldScale3D` (`self.Decal`) (`KismetMathLibrary.Conv_DoubleToVector` _decalsize))))))
    (else
      (goto _label))))

(fn `UserConstructionScript`)