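; Height-capture actor for terrain deformation that follows the player character, or a bulldozer when none is valid, with an orthographic scene capture.
; Each tick it moves by an offset computed through a pixel-grid snap function and publishes its location to a material parameter collection.
; It then draws materials into persistent and blurred final render targets, passing the normalized move offset so they can account for the scrolling window.
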(event `self.ReceiveBeginPlay`
  (`KismetMaterialLibrary.SetScalarParameterValue` "/Game/ConstructionSite/Effects/TerrainDeformation_01/Materials/mpc_CaptureHeight_01_01.mpc_CaptureHeight_01_01" "CaptureSize" (`SceneCaptureComponent2D.OrthoWidth` (`self.SceneCapture`)))
  (bind _returnvalue (`KismetMaterialLibrary.CreateDynamicMaterialInstance` "/Game/ConstructionSite/Effects/TerrainDeformation_01/Materials/m_DrawToPersistent_01_01.m_DrawToPersistent_01_01"))
  (set `self.DrawMaterial` _returnvalue)
  (bind _returnvalue_2 (`KismetMaterialLibrary.CreateDynamicMaterialInstance` "/Game/ConstructionSite/Effects/TerrainDeformation_01/Materials/m_DrawBlurToFinal_01_01.m_DrawBlurToFinal_01_01"))
  (set `self.DrawBlurMaterial` _returnvalue_2)
  (`KismetRenderingLibrary.ClearRenderTarget2D` "/Game/ConstructionSite/Effects/TerrainDeformation_01/RenderTargets/rt_Capture_01_01.rt_Capture_01_01")
  (`KismetRenderingLibrary.ClearRenderTarget2D` "/Game/ConstructionSite/Effects/TerrainDeformation_01/RenderTargets/rt_Persistent_01_01.rt_Persistent_01_01")
  (`KismetRenderingLibrary.ClearRenderTarget2D` "/Game/ConstructionSite/Effects/TerrainDeformation_01/RenderTargets/rt_Final_01_01.rt_Final_01_01"))

(event `self.ReceiveTick`
  (params (DeltaSeconds :type "Float (single-precision)"))
  (`self.MoveCapture`)
  (`self.DrawToPersistent`)
  (`self.DrawBlurToFinal`))

(fn `DrawBlurToFinal`
  (bind (_returnvalue_x _returnvalue_y) (`KismetMathLibrary.BreakVector2D` (/ (`self.MoveOffset`) (`SceneCaptureComponent2D.OrthoWidth` (`self.SceneCapture`)))))
  (`MaterialInstanceDynamic.SetVectorParameterValue` (`self.DrawBlurMaterial`) "Offset" (make `LinearColor` _returnvalue_x _returnvalue_y 0.0 1.0))
  (`KismetRenderingLibrary.DrawMaterialToRenderTarget` "/Game/ConstructionSite/Effects/TerrainDeformation_01/RenderTargets/rt_Final_01_01.rt_Final_01_01" (`self.DrawBlurMaterial`)))

(fn `DrawToPersistent`
  (bind (_returnvalue_x _returnvalue_y) (`KismetMathLibrary.BreakVector2D` (/ (`self.MoveOffset`) (`SceneCaptureComponent2D.OrthoWidth` (`self.SceneCapture`)))))
  (`MaterialInstanceDynamic.SetVectorParameterValue` (`self.DrawMaterial`) "Offset" (make `LinearColor` _returnvalue_x _returnvalue_y 0.0 1.0))
  (`KismetRenderingLibrary.DrawMaterialToRenderTarget` "/Game/ConstructionSite/Effects/TerrainDeformation_01/RenderTargets/rt_Persistent_01_01.rt_Persistent_01_01" (`self.DrawMaterial`)))

(fn `MoveCapture`
  (bind _returnvalue (`GameplayStatics.GetPlayerCharacter` 0))
  (bind (_playerposition_x _playerposition_y) (`KismetMathLibrary.BreakVector` (`self.PlayerPosition`)))
  (bind (_returnvalue_x _returnvalue_y) (`KismetMathLibrary.BreakVector` (- (`self.SnapToPixelWorldSize` _playerposition_x _playerposition_y (* (`SceneCaptureComponent2D.OrthoWidth` (`self.SceneCapture`)) (/ 1.0 2048.0))) (`self.K2_GetActorLocation`))))
  (`/Engine/EditorBlueprintResources/StandardMacros.IsValid` _returnvalue
    (:`Is Valid`
      (set `self.PlayerPosition` (`self.K2_GetActorLocation` _returnvalue)))
    (:`Is Not Valid`
      (bind _outactors (`GameplayStatics.GetAllActorsOfClass` "/Game/ConstructionSite/Vehicle/Bulldozer_01/bp_Bulldozer_01_01.BP_Bulldozer_01_01_C"))
      (bind _output (`|GetArrayItem` _outactors))
      (`/Engine/EditorBlueprintResources/StandardMacros.IsValid` _output
        (:`Is Valid`
          (set `self.PlayerPosition` (`self.K2_GetActorLocation` _output))))))
  (bind _output_get (set `self.MoveOffset` (`KismetMathLibrary.MakeVector2D` _returnvalue_x _returnvalue_y)))
  (`self.K2_AddActorWorldOffset` (`KismetMathLibrary.MakeVector` (`KismetMathLibrary.BreakVector2D` _output_get) (`.Y` (`KismetMathLibrary.BreakVector2D` _output_get))))
  (`KismetMaterialLibrary.SetVectorParameterValue` "/Game/ConstructionSite/Effects/TerrainDeformation_01/Materials/mpc_CaptureHeight_01_01.mpc_CaptureHeight_01_01" "CaptureLocation" (`KismetMathLibrary.Conv_VectorToLinearColor` (`self.K2_GetActorLocation`))))

(fn `UserConstructionScript`)